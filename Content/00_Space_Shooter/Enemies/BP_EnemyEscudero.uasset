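; BP_EnemyEscudero is a space shooter enemy built on a parent Blueprint, with its lives (Vidas) set to five in the construction script.
; On BeginPlay it sets MovementVector once from the player's position relative to a fixed point, not its own location, normalized and then flattened to XY.
; It has no active Tick or overlap logic of its own.
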(event `self.ReceiveBeginPlay`
  (`parent.ReceiveBeginPlay`)
  (set `self.MovementVector` (* (`KismetMathLibrary.Normal` (- (-1.0 -1.0 0.0) (`SceneComponent.K2_GetComponentLocation` (`Actor.RootComponent` (`GameplayStatics.GetPlayerCharacter` 0))))) (-1.0 -1.0 0.0))))

(fn `UserConstructionScript`
  (`parent.UserConstructionScript`)
  (set `self.Vidas` 5))
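; Space shooter follower enemy that heads toward the player and can fire, extending a parent enemy class.
; On BeginPlay it calls the parent, then sets MovementVector once from its SMArrows position toward the player, flattened in Z.
; It also starts a timer with no visible function name, zeroes ShootCurrentTime and calls Fire only if that exceeds DelayShoot.
; Tick and overlap events are disabled stubs, so this graph never re-aims.
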(event `self.ReceiveBeginPlay`
  (`parent.ReceiveBeginPlay`)
  (set `self.MovementVector` (* (`KismetMathLibrary.Normal` (- (`SceneComponent.K2_GetComponentLocation` (`self.SM_Arrows`)) (`SceneComponent.K2_GetComponentLocation` (`Actor.RootComponent` (`GameplayStatics.GetPlayerCharacter` 0))))) (-10.0 -10.0 0.0)))
  (`KismetSystemLibrary.K2_SetTimer` null)
  (set `self.ShootCurrentTime` 0.0)
  (if (> (`self.ShootCurrentTime`) (`self.DelayShoot`))
    (`self.Fire`)))

(fn `UserConstructionScript`
  (`parent.UserConstructionScript`))